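; BP_TyrantBear is an enemy pawn that chases the player and restarts the current level when it overlaps them.
; BeginPlay sets actor tick from the AutoActivate flag, so the chase runs from the start only when that flag is on.
; While ticking, it reissues AIMoveTo toward the player character every frame.
; Overlap with the player reopens the level by its current name, independently of the tick logic.
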(event `self.ReceiveBeginPlay`
  (`parent.ReceiveBeginPlay`)
  (`self.SetActorTickEnabled` (`self.Auto Activate`)))

(event `self.ReceiveActorBeginOverlap`
  (params (OtherActor :type "Actor Object Reference"))
  (if (== OtherActor (`GameplayStatics.GetPlayerCharacter` 0))
    (bind _returnvalue (`GameplayStatics.GetCurrentLevelName` true))
    (`GameplayStatics.OpenLevel` (`KismetStringLibrary.Conv_StringToName` _returnvalue))))

(event `self.ReceiveTick`
  (params (DeltaSeconds :type "Float (single-precision)"))
  (`|AIMoveTo` self (0.0 0.0 0.0) (`GameplayStatics.GetPlayerCharacter` 0)))

(fn `UserConstructionScript`
  (`parent.UserConstructionScript`))