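; BP_UnhideTrigger is a one-shot overlap trigger that reveals a referenced actor during play.
; On BeginPlay it hides that UnhideBP actor and disables its tick and collision.
; When TriggeredByBP, or the player character if that reference is unset, overlaps it, it restores visibility, tick and collision on the target and destroys itself.
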(event `self.ReceiveBeginPlay`
  (`self.SetActorHiddenInGame` (`self.Unhide_BP`) true)
  (`self.SetActorTickEnabled` (`self.Unhide_BP`) false)
  (`self.SetActorEnableCollision` (`self.Unhide_BP`) false))

(event `self.ReceiveActorBeginOverlap`
  (params (OtherActor :type "Actor Object Reference"))
  (bind _triggeredby_bp (`self.TriggeredBy_BP`))
  (bind _unhide_bp (`self.Unhide_BP`))
  (`/Engine/EditorBlueprintResources/StandardMacros.IsValid` _triggeredby_bp
    (:`Is Valid`
      (if (== OtherActor _triggeredby_bp)
        (`self.SetActorHiddenInGame` _unhide_bp false :!label _label)
        (`self.SetActorTickEnabled` _unhide_bp true)
        (`self.SetActorEnableCollision` (`self.Unhide_BP`) true)
        (`self.K2_DestroyActor`)))
    (:`Is Not Valid`
      (if (== OtherActor (`GameplayStatics.GetPlayerCharacter` 0))
        (goto _label)))))

(fn `UserConstructionScript`)